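; Proof-of-concept player controller holding debug hotkeys to test looting, merchant trading and inventory UI refresh.
; L and M keys, with Ctrl variants, fire once per press into server-named events targeting the first or second lootable or merchant found by GetAllActorsOfClass.
; Those events check the current looting or trading state, plus whether a lootable is taken, before calling ServerLootActor or ServerMerchantTrade.
; T refreshes all main HUD inventory grids.
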(event Custom|ServerSelectLootable2
  ;[1 1 1] DEBUG FUNCTIONS
  (if (not (Class|MainPlayerController|IsLooting))
    (bind _outactors (Actor|GetAllActorsOfClass "/Game/POC/Actors/BP_LootableActor.BP_LootableActor_C"))
    (Utilities|IsValid (Utilities|Array|Get(acopy) _outactors 1)
      (:Is%20Valid
        (if (Variables|/Script/InventoryPOC.LootableActor|GetIsBeingLooted (Utilities|Array|Get(acopy) _outactors 1))
          (Development|PrintString "Actor is already being looted")
          (else
            (Class|MainPlayerController|ServerLootActor (Utilities|Array|Get(acopy) _outactors 1))
            (Development|PrintString "Looting new actor")))))
    (else
      (Development|PrintString "Already looting"))))

(event Custom|Server_SelectMerchant2
  ;[1 1 1] DEBUG FUNCTIONS
  (if (not (Class|MainPlayerController|IsTrading))
    (bind _outactors (Actor|GetAllActorsOfClass "/Game/POC/Actors/BP_MerchantActor.BP_MerchantActor_C"))
    (Utilities|IsValid (Utilities|Array|Get(acopy) _outactors 1)
      (:Is%20Valid
        (Class|MainPlayerController|ServerMerchantTrade (Utilities|Array|Get(acopy) _outactors 1))
        (Development|PrintString "Starting merchant trade")))))

(event Custom|Server_SelectMerchant
  ;[1 1 1] DEBUG FUNCTIONS
  (if (not (Class|MainPlayerController|IsTrading))
    (bind _outactors (Actor|GetAllActorsOfClass "/Game/POC/Actors/BP_MerchantActor.BP_MerchantActor_C"))
    (Utilities|IsValid (Utilities|Array|Get(acopy) _outactors)
      (:Is%20Valid
        (Class|MainPlayerController|ServerMerchantTrade (Utilities|Array|Get(acopy) _outactors))
        (Development|PrintString "Starting merchant trade")))))

(event Custom|Server_SelectLootable
  ;[1 1 1] DEBUG FUNCTIONS
  (if (not (Class|MainPlayerController|IsLooting))
    (bind _outactors (Actor|GetAllActorsOfClass "/Game/POC/Actors/BP_LootableActor.BP_LootableActor_C"))
    (Utilities|IsValid (Utilities|Array|Get(acopy) _outactors)
      (:Is%20Valid
        (if (Variables|/Script/InventoryPOC.LootableActor|GetIsBeingLooted (Utilities|Array|Get(acopy) _outactors))
          (Development|PrintString "Actor is already being looted")
          (else
            (Class|MainPlayerController|ServerLootActor (Utilities|Array|Get(acopy) _outactors))
            (Development|PrintString "Looting new actor")))))
    (else
      (Development|PrintString "Already looting"))))

(event EventBeginPlay)

(event EventTick
  (params (DeltaSeconds :type Float%20%28single-precision%29)))

(event Input|KeyboardEvents|T
  (params (Key :type Key%20Structure :default "None"))
  ;[1 1 1] DEBUG FUNCTIONS
  (:Pressed
    (Development|PrintString "Hello")
    (bind _returnvalue (Class|MainPlayerController|GetMainHUD))
    (Class|HUDWidget|RefreshAllInventoryGrids _returnvalue)))

(event Input|KeyboardEvents|CtrlL
  (params (Key :type Key%20Structure :default "None"))
  ;[1 1 1] DEBUG FUNCTIONS
  (:Pressed
    (Utilities|FlowControl|DoOnce false :!label _label
      (:Completed
        (Development|PrintString "Hello")
        (CallFunction|ServerSelectLootable2))))
  (:Released
    (goto _label Reset)))

(event Input|KeyboardEvents|CtrlM
  (params (Key :type Key%20Structure :default "None"))
  ;[1 1 1] DEBUG FUNCTIONS
  (:Pressed
    (Utilities|FlowControl|DoOnce false :!label _label
      (:Completed
        (CallFunction|ServerSelectMerchant2))))
  (:Released
    (goto _label Reset)))

(event Input|KeyboardEvents|M
  (params (Key :type Key%20Structure :default "None"))
  ;[1 1 1] DEBUG FUNCTIONS
  (:Pressed
    (Utilities|FlowControl|DoOnce false :!label _label
      (:Completed
        (CallFunction|ServerSelectMerchant))))
  (:Released
    (goto _label Reset)))

(event Input|KeyboardEvents|L
  (params (Key :type Key%20Structure :default "None"))
  ;[1 1 1] DEBUG FUNCTIONS
  (:Pressed
    (Utilities|FlowControl|DoOnce false :!label _label
      (:Completed
        (Development|PrintString "Hello")
        (CallFunction|ServerSelectLootable))))
  (:Released
    (goto _label Reset)))

(fn ConstructionScript)